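; BP_Ball is the player-controlled rolling ball, which handles its own movement and death.
; Forward/backward and left/right axis inputs apply scaled acceleration-change torque to ShapeSphere, so it moves through physics.
; The first damage of any amount is fatal: a DoOnce shows the YourDead widget, then after delays clears widgets, fades the camera and reloads the current level.
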(event EventBeginPlay)

(event Collision|EventActorBeginOverlap
  (params (OtherActor :type Actor%20Object%20Reference)))

(event EventTick
  (params (DeltaSeconds :type Float%20%28single-precision%29)))

(event Game|Damage|EventAnyDamage
  (params (Damage :type Float%20%28single-precision%29) (DamageType :type Damage%20Type%20Object%20Reference) (InstigatedBy :type Controller%20Object%20Reference) (DamageCauser :type Actor%20Object%20Reference))
  (Utilities|FlowControl|DoOnce false
    (:Completed
      (bind _returnvalue (UserInterface|CreateWidget (Variables|Default|Getyour%20dead)))
      (UserInterface|Viewport|AddtoViewport _returnvalue 0)
      (Utilities|FlowControl|Delay 2.5)
      (Viewport|RemoveAllWidgets)
      (CameraFades|StartCameraFade :self (Game|GetPlayerCameraManager 0) :ToAlpha 5.0 :Duration 5.0)
      (Utilities|FlowControl|Delay 2.5)
      (bind _returnvalue_2 (Game|GetCurrentLevelName true))
      (Game|OpenLevel(byName) (Utilities|String|StringToName _returnvalue_2)))))

(event Input|AxisEvents|InputAxisMoveforwards/backwards
  (params (AxisValue :type Float%20%28single-precision%29))
  (Class|PrimitiveComponent|AddTorqueinRadians (Variables|Default|GetShape_Sphere) (Math|Vector|MakeVector 0.0 (* AxisValue (Variables|Default|Getaxis_multi)) 0.0) "None" true))

(event Input|AxisEvents|InputAxisleft/right
  (params (AxisValue :type Float%20%28single-precision%29))
  (Class|PrimitiveComponent|AddTorqueinRadians (Variables|Default|GetShape_Sphere) (Math|Vector|MakeVector (* AxisValue (Variables|Default|Getaxis_multi)) 0.0 0.0) "None" true))

(fn ConstructionScript)