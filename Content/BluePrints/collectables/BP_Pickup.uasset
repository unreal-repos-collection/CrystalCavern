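; BP_Pickup is a collectable crystal with a point light that plays a collection animation when the player pawn overlaps it, then destroys itself.
; On overlap it stores its starting location, scale and light intensity.
; A timeline then drives three lerps from those values, pulling the crystal toward the player's current position while shrinking it and fading its light to zero.
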(event Collision|EventActorBeginOverlap
  (params (OtherActor :type Actor%20Object%20Reference))
  (Utilities|IsPlayer OtherActor
    (:is%20player
      (CallFunction|StoreStartingValues)
      (bind (_direction _collection_progress _scale_progress _light_intensity) (Timeline|Collection%20timeline Play)
        (:Update
          (CallFunction|MovetoPlayer _collection_progress)
          (CallFunction|ScaleCrystal _scale_progress)
          (CallFunction|LightScale _light_intensity))
        (:Finished
          (Actor|DestroyActor))))))

(fn ConstructionScript)

(fn MovetoPlayer
  (params (Alpha :type Float%20%28single-precision%29))
  (Transformation|SetActorLocation (Math|Vector|Lerp(Vector) (Variables|Default|GetStart) (Transformation|GetActorLocation (Game|Player|GetPlayerPawn 0)) Alpha) false false))

(fn StoreStartingValues
  (Variables|Default|SetStart (Transformation|GetActorLocation))
  (Variables|Default|Setstartscale (Transformation|GetActorScale3D))
  (Variables|Default|Setstartlightintensity (Variables|/Script/Engine.LightComponentBase|GetIntensity (Variables|Default|GetPointLight))))

(fn ScaleCrystal
  (params (Alpha :type Float%20%28single-precision%29))
  (Transformation|SetActorScale3D (Math|Vector|Lerp(Vector) (Variables|Default|Getstartscale) "0, 0, 0" Alpha)))

(fn LightScale
  (params (Alpha :type Float%20%28single-precision%29))
  (Rendering|Components|Light|SetIntensity (Variables|Default|GetPointLight) (Math|Float|Lerp (Variables|Default|Getstartlightintensity) 0.0 Alpha)))